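; Base enemy Blueprint driven by an AI Controller that reports to its Spawner when destroyed.
; Capsule overlaps with BP_Node actors, ignoring their "Box" component and the first node in LastPositions, append the node to that list and write it to the AI blackboard.
; Desintegrate is a placeholder that only prints a debug message, and overlaps also print the component name.
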(event OnComponentBeginOverlap(CapsuleComponent)
  (params (OverlappedComponent :type Primitive%20Component%20Object%20Reference) (OtherActor :type Actor%20Object%20Reference) (OtherComp :type Primitive%20Component%20Object%20Reference) (OtherBodyIndex :type Integer) (bFromSweep :type Boolean) (SweepResult :type Hit%20Result%20Structure%20%28by%20ref%29))
  (bind _lastpositions (Variables|Positions|GetLastPositions))
  (Development|PrintString (Utilities|GetDisplayName OtherComp))
  (bind _asbp_node (Utilities|Casting|CastToBP_Node OtherActor))
  (if (and (not (Utilities|Enum|Equal(Enum) (Utilities|GetObjectName OtherComp) "Box")) (!= _asbp_node (Utilities|Array|Get(acopy) _lastpositions)))
    (Utilities|Array|Add _lastpositions _asbp_node)
    (AI|Components|Blackboard|SetValueasObject (AI|GetBlackboard (Variables|Default|GetAIController)) (Variables|Default|GetNewVar_1) _asbp_node)))

(event EventTick
  (params (DeltaSeconds :type Float%20%28single-precision%29)))

(event EventEndPlay
  (params (EndPlayReason :type EEndPlayReason%20Enum :default "Destroyed"))
  (switch Utilities|FlowControl|Switch|SwitchonEEndPlayReason EndPlayReason
    (:Destroyed
      (Default|EnemyDestroyed (Variables|SpawnerOwner|GetSpawner)))))

(event EventBeginPlay
  (bind _asaicontroller (Utilities|Casting|CastToAIController (Pawn|GetController)))
  (Variables|Default|SetAIController _asaicontroller))

(fn ConstructionScript)

(fn Desintegrate
  (Development|PrintString "Me estoy desintegrando"))