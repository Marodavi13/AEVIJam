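; Input-handling pawn that turns clicks into interactions with the world and selects one of three skills (Nuke, BinaryRay, Decoy).
; TraceforBlock stores the actor hit by a visibility line trace, and LeftClick sends it InteractMessage through BP_InteractionInterface.
; ActivateSkill stores the chosen skill, but the game-state branch that would pass it to the actor is disconnected.
; Zoom, rotate, move and right-click events are empty stubs.
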(event EventBeginPlay)

(event Collision|EventActorBeginOverlap
  (params (OtherActor :type Actor%20Object%20Reference)))

(event EventTraceforBlock
  (params (Start :type Vector%20%28by%20ref%29 :default "0, 0, 0") (End :type Vector%20%28by%20ref%29 :default "0, 0, 0") (bDrawDebugHelpers :type Boolean))
  (bind (_outhit _returnvalue) (Collision|LineTraceByChannel Start End "TraceTypeQuery1" false 0 "None"))
  (if _returnvalue
    (Variables|Default|SetActor (.hitactor _outhit))))

(event EventTick
  (params (DeltaSeconds :type Float%20%28single-precision%29)))

(event EventZoomOut)

(event EventRotateMap
  (params (Value :type Float%20%28single-precision%29)))

(event EventMoveVertical
  (params (Value :type Float%20%28single-precision%29)))

(event EventLeftClick
  (bind _actor (Variables|Default|GetActor))
  (bind _asbp_aevijam_controller (Utilities|Casting|CastToBP_AEVIJamController (Pawn|GetController)))
  (if (Utilities|DoesObjectImplementInterface _actor "/Game/AEVIContent/Interfaces/BP_InteractionInterface.BP_InteractionInterface_C")
    (Class|BPInteractionInterface|Interact(Message) _actor)))

(event EventZoomin)

(event EventRightClick
  (params (ButtonAction :type EInputEvent%20Enum :default "IE_Pressed")))

(event EventMoveHorizontal
  (params (Value :type Float%20%28single-precision%29)))

(event EventActivateSkill
  (params (NumberOfSkill :type Integer))
  (switch int NumberOfSkill
    (:1
      (Variables|Default|SetActivatedSkill "/Game/AEVIContent/Skillz/BP_SkillNuke.BP_SkillNuke_C"))
    (:2
      (Variables|Default|SetActivatedSkill "/Game/AEVIContent/Skillz/BP_SkillBinaryRay.BP_SkillBinaryRay_C"))
    (:3
      (Variables|Default|SetActivatedSkill "/Game/AEVIContent/Skillz/BP_SkillDecoy.BP_SkillDecoy_C"))))

(fn ConstructionScript)