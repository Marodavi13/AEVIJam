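; BP_SkillNuke is a skill that, on activation, instantly wipes out every enemy in its target Node.
; The Node can be a BP_Room or a BP_Connection, each supplying its own box collision as the kill area.
; Every BP_EnemyBase overlapping that box is destroyed outright with DestroyActor, iterating in reverse and applying no damage.
; An invalid Node or any other node type does nothing.
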(event EventActivateSkill
  (bind _node (Variables|Default|GetNode))
  (Utilities|IsValid _node
    (:Is%20Valid
      (Utilities|Casting|CastToBP_Room _node
        (:then
          (bind _arrayelement (Utilities|Array|ReverseforEachLoop (Collision|GetOverlappingActors (Variables|/Game/AEVIContent/Nodes/BP_Room.BP_Room_C|GetBox%20Collision _node) "/Game/AEVIContent/Enemies/BP_EnemyBase.BP_EnemyBase_C" :!class /Script/Engine.PrimitiveComponent))
            (:LoopBody
              (Actor|DestroyActor _arrayelement))))
        (:CastFailed
          (bind _asbp_connection (Utilities|Casting|CastToBP_Connection _node))
          (bind _arrayelement_2 (Utilities|Array|ReverseforEachLoop (Collision|GetOverlappingActors (Variables|/Game/AEVIContent/Nodes/BP_Connection.BP_Connection_C|GetBox _asbp_connection) "/Game/AEVIContent/Enemies/BP_EnemyBase.BP_EnemyBase_C" :!class /Script/Engine.PrimitiveComponent))
            (:LoopBody
              (Actor|DestroyActor _arrayelement_2))))))))