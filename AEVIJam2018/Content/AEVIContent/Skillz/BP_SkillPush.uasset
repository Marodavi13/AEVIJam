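; BP_SkillPush is a skill that pushes enemies in a room or connection back toward places they recently occupied.
; On activation it gathers enemies overlapping the Node's box collision, using identical logic for BP_Room and BP_Connection.
; Each enemy with enough LastPositions history is launched toward the entry at PushBackPositions - 1.
; Launch velocity is displacement over LaunchTime, with the acceleration term zeroed, so gravity is not compensated.
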(event EventActivateSkill
  (bind _launchtime (Variables|Default|GetLaunchTime))
  (bind _launchtime_2 (Variables|Default|GetLaunchTime))
  (bind _pushbackpositions (Variables|Default|GetPushBackPositions))
  (bind _node (Variables|Default|GetNode))
  (bind _pushbackpositions_2 (Variables|Default|GetPushBackPositions))
  (bind _returnvalue (- _pushbackpositions_2 1))
  (bind _returnvalue_2 (- _pushbackpositions 1))
  (bind _box_collision (Variables|/Game/AEVIContent/Nodes/BP_Node.BP_Node_C|GetBox%20Collision _node))
  (Utilities|IsValid _node
    (:Is%20Valid
      (Utilities|Casting|CastToBP_Room _node
        (:then
          (bind _arrayelement (Utilities|Array|ReverseforEachLoop (Collision|GetOverlappingActors _box_collision "/Game/AEVIContent/Enemies/BP_EnemyBase.BP_EnemyBase_C" :!class /Script/Engine.PrimitiveComponent))
            (:LoopBody
              (bind _asbp_enemy_base (Utilities|Casting|CastToBP_EnemyBase _arrayelement))
              (if (Utilities|Array|IsValidIndex (Variables|/Game/AEVIContent/Enemies/BP_EnemyBase.BP_EnemyBase_C|GetLastPositions _asbp_enemy_base) _returnvalue)
                (Character|LaunchCharacter _asbp_enemy_base (- (/ (- (Transformation|GetActorLocation (Utilities|Array|Get(acopy) (Variables|/Game/AEVIContent/Enemies/BP_EnemyBase.BP_EnemyBase_C|GetLastPositions _asbp_enemy_base) _returnvalue)) (Transformation|GetActorLocation _arrayelement)) _launchtime) (* (* "0, 0, 0" _launchtime) 0.5)) false false)))))
        (:CastFailed
          (Utilities|Casting|CastToBP_Connection _node)
          (bind _arrayelement_2 (Utilities|Array|ReverseforEachLoop (Collision|GetOverlappingActors _box_collision "/Game/AEVIContent/Enemies/BP_EnemyBase.BP_EnemyBase_C" :!class /Script/Engine.PrimitiveComponent))
            (:LoopBody
              (bind _asbp_enemy_base_2 (Utilities|Casting|CastToBP_EnemyBase _arrayelement_2))
              (if (Utilities|Array|IsValidIndex (Variables|/Game/AEVIContent/Enemies/BP_EnemyBase.BP_EnemyBase_C|GetLastPositions _asbp_enemy_base_2) _returnvalue_2)
                (Character|LaunchCharacter _asbp_enemy_base_2 (- (/ (- (Transformation|GetActorLocation (Utilities|Array|Get(acopy) (Variables|/Game/AEVIContent/Enemies/BP_EnemyBase.BP_EnemyBase_C|GetLastPositions _asbp_enemy_base_2) _returnvalue_2)) (Transformation|GetActorLocation _arrayelement_2)) _launchtime_2) (* (* "0, 0, 0" _launchtime_2) 0.5)) false false)))))))))