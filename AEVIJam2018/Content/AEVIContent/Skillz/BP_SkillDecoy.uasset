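; Decoy skill that briefly switches on a sphere on its target Node, which is either a room or a connection.
; Activation reveals that node's Sphere and enables its query and physics collision, then a timer calls StopSkill after a few seconds to hide and disable it.
; Enemies overlapping the node's BoxCollision only have their names printed; no decoy effect is applied to them here.
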(event Custom|StopSkill
  (bind _node (Variables|Default|GetNode))
  (bind _sphere (Variables|/Game/AEVIContent/Nodes/BP_Node.BP_Node_C|GetSphere _node))
  (Development|SetHiddeninGame _sphere true false)
  (Collision|SetCollisionEnabled _sphere "NoCollision"))

(event EventActivateSkill
  (bind _node (Variables|Default|GetNode))
  (bind _sphere (Variables|/Game/AEVIContent/Nodes/BP_Node.BP_Node_C|GetSphere _node))
  (bind _sphere_2 (Variables|/Game/AEVIContent/Nodes/BP_Node.BP_Node_C|GetSphere _node))
  (Utilities|IsValid _node
    (:Is%20Valid
      (Utilities|Casting|CastToBP_Room _node
        (:then
          (Development|SetHiddeninGame _sphere_2 false false)
          (Collision|SetCollisionEnabled _sphere_2 "QueryAndPhysics")
          (bind _arrayelement (Utilities|Array|ReverseforEachLoop (Collision|GetOverlappingActors (Variables|/Game/AEVIContent/Nodes/BP_Node.BP_Node_C|GetBox%20Collision _node) "/Game/AEVIContent/Enemies/BP_EnemyBase.BP_EnemyBase_C" :!class /Script/Engine.PrimitiveComponent))
            (:LoopBody
              (Development|PrintString 0 (Utilities|GetDisplayName _arrayelement)))
            (:Completed
              (Utilities|Time|SetTimerbyEvent (delegate Custom|StopSkill) 4.0 :!label _label))))
        (:CastFailed
          (Utilities|Casting|CastToBP_Connection _node)
          (Development|SetHiddeninGame _sphere false false)
          (Collision|SetCollisionEnabled _sphere "QueryAndPhysics")
          (bind _arrayelement_2 (Utilities|Array|ReverseforEachLoop (Collision|GetOverlappingActors (Variables|/Game/AEVIContent/Nodes/BP_Node.BP_Node_C|GetBox%20Collision _node) "/Game/AEVIContent/Enemies/BP_EnemyBase.BP_EnemyBase_C" :!class /Script/Engine.PrimitiveComponent))
            (:LoopBody
              (Development|PrintString 0 (Utilities|GetDisplayName _arrayelement_2)))
            (:Completed
              (goto _label))))))))