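; Binary Ray skill that, on activation, randomly wipes out one of two enemy types at the target node.
; It accepts the Node as either a room or a connection and queries that node's box collision for overlaps.
; A roughly even random roll picks BP_Enemy0 or BP_Enemy1, and every overlapping actor of that class is destroyed, iterating in reverse.
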(event EventActivateSkill
  (bind _node (Variables|Default|GetNode))
  (bind _box_collision (Variables|/Game/AEVIContent/Nodes/BP_Room.BP_Room_C|GetBox%20Collision _node))
  (bind _box_collision_2 (Variables|/Game/AEVIContent/Nodes/BP_Room.BP_Room_C|GetBox%20Collision _node))
  (Utilities|IsValid _node
    (:Is%20Valid
      (Utilities|Casting|CastToBP_Room _node
        (:then
          (if (<= (Math|Random|RandomIntegerinRange 1 100) 50)
            (bind _arrayelement (Utilities|Array|ReverseforEachLoop (Collision|GetOverlappingActors _box_collision_2 "/Game/AEVIContent/Enemies/BP_Enemy0.BP_Enemy0_C" :!class /Script/Engine.PrimitiveComponent))
              (:LoopBody
                (Actor|DestroyActor _arrayelement)))
            (else
              (bind _arrayelement_2 (Utilities|Array|ReverseforEachLoop (Collision|GetOverlappingActors _box_collision_2 "/Game/AEVIContent/Enemies/BP_Enemy1.BP_Enemy1_C" :!class /Script/Engine.PrimitiveComponent))
                (:LoopBody
                  (Actor|DestroyActor _arrayelement_2))))))
        (:CastFailed
          (Utilities|Casting|CastToBP_Connection _node)
          (if (<= (Math|Random|RandomIntegerinRange 1 100) 50)
            (bind _arrayelement_3 (Utilities|Array|ReverseforEachLoop (Collision|GetOverlappingActors _box_collision "/Game/AEVIContent/Enemies/BP_Enemy0.BP_Enemy0_C" :!class /Script/Engine.PrimitiveComponent))
              (:LoopBody
                (Actor|DestroyActor _arrayelement_3)))
            (else
              (bind _arrayelement_4 (Utilities|Array|ReverseforEachLoop (Collision|GetOverlappingActors _box_collision "/Game/AEVIContent/Enemies/BP_Enemy1.BP_Enemy1_C" :!class /Script/Engine.PrimitiveComponent))
                (:LoopBody
                  (Actor|DestroyActor _arrayelement_4))))))))))