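; BP_GridManager builds a rectangular grid of child actors, apparently for a game board.
; Its Construction Script adds one child actor component per cell from the row and column counts, spacing them by Width on X and Y.
; Each component is stored in GridArray; the final loop over that array is empty, and the event graph has no logic.
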(event EventBeginPlay)

(event Collision|EventActorBeginOverlap
  (params (OtherActor :type Actor%20Object%20Reference)))

(event EventTick
  (params (DeltaSeconds :type Float%20%28single-precision%29)))

(fn ConstructionScript
  (LocalVariables|SetCurrentRow 0)
  (LocalVariables|SetCurrentColumn 0)
  (bind _output_get (LocalVariables|SetGridsRemaining (* (Variables|Default|GetNumberOfRows) (Variables|Default|GetNumberOfColumns))))
  (while (> _output_get 0)
    (Math|Integer|DecrementInt (LocalVariables|GetGridsRemaining)
      (:%20%20
        (bind _returnvalue (AddComponent|AddChildActorComponent false (Math|Transform|MakeTransform (Math|Vector|MakeVector (Math|Conversions|ToFloat(Integer) (* (LocalVariables|GetCurrentRow) (Variables|Default|GetWidth))) (Math|Conversions|ToFloat(Integer) (* (LocalVariables|GetCurrentColumn) (Variables|Default|GetWidth))) 0.0) "0, 0, 0" "1,1,1")))
        (Utilities|Array|AddUnique (Variables|Default|GetGridArray) _returnvalue)
        (bind _result (Math|Integer|IncrementInt (LocalVariables|GetCurrentColumn))
          (:%20%20
            (if (>= _result (Variables|Default|GetNumberOfColumns))
              (LocalVariables|SetCurrentColumn 0)
              (Math|Integer|IncrementInt (LocalVariables|GetCurrentRow))))))))
  (for _array_element (Variables|Default|GetGridArray)
    _))