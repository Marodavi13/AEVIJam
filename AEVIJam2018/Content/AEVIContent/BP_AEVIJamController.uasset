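; BP_AEVIJamController controls the game loop, switching GameState between phases such as Defending and Respecting.
; SetGameState starts a level on the first BP_SpawnsManager found when Defending begins, then increments Level.
; Respecting schedules the return to Defending on a timer whose duration is read from a float curve by Level.
; Tick prints the current state as debug output; BeginPlay, StartState and Foo are stubs or test code.
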(event EventBeginPlay)

(event EventTick
  (params (DeltaSeconds :type Float%20%28single-precision%29))
  (Development|PrintString (Utilities|String|Append "GAME STATE:" (Utilities|String|EnumtoString (Variables|Default|GetGameState))) true true "(R=0.000000,G=0.660000,B=1.000000,A=1.000000)" DeltaSeconds))

(fn ConstructionScript)

(fn SetGameState
  (params (NewGameState :type EGameState%20Enum :default "NewEnumerator2"))
  (bind _output_get (Variables|Default|SetGameState NewGameState))
  (switch Utilities|FlowControl|Switch|SwitchonEGameState _output_get
    (:NewEnumerator0
      (bind _outactors (Actor|GetAllActorsOfClass "/Game/AEVIContent/Spawn/BP_SpawnsManager.BP_SpawnsManager_C"))
      (bind _asbp_spawns_manager (Utilities|Casting|CastToBP_SpawnsManager (Utilities|Array|Get(acopy) _outactors)))
      (Default|StartLevel _asbp_spawns_manager)
      (Math|Integer|IncrementInt (Variables|Default|GetLevel)))
    (:NewEnumerator1
      (Utilities|Time|SetTimerbyFunctionName 0 "SetDefendingState" (Math|Curves|GetFloatValue (Variables|Default|GetCF_TimeRespecting) (Math|Conversions|ToFloat(Integer) (Variables|Default|GetLevel)))))))

(fn StartState)

(fn Foo
  (Development|PrintString "Hello"))

(fn SetDefendingState
  (CallFunction|SetGameState "NewEnumerator0"))