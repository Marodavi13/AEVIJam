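; Spawn manager that runs level-based enemy waves across all BP_Spawner actors, registering itself with each on BeginPlay.
; StartLevel samples float curves at CurrentLevel for wave count, enemy count, added speed and timings, then starts every spawner and shows the start widget.
; Spawners report back through SpawnLevelFinished, which updates per-spawner active flags, calls LevelFinished for game state and end-level UI, and increments CurrentLevel.
; Tick prints CurrentLevel for debugging.
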(event EventBeginPlay
  (Variables|Default|SetCurrentLevel 1.0)
  (Utilities|Array|Clear (Variables|Default|GetSpawns))
  (bind _outactors (Actor|GetAllActorsOfClass "/Game/AEVIContent/Spawn/BP_Spawner.BP_Spawner_C"))
  (bind _output_get (Variables|Default|SetSpawns _outactors))
  (for (_array_element _array_index) _output_get
    (Variables|/Game/AEVIContent/Spawn/BP_Spawner.BP_Spawner_C|SetSpawnManager _array_element self)
    (Utilities|Array|SetArrayElem (Variables|Default|GetbAreLevelsActiveArray) _array_index true true))
  (bind _asbp_aevijam_controller (Utilities|Casting|CastToBP_AEVIJamController (Game|GetPlayerController 0))))

(event EventTick
  (params (DeltaSeconds :type Float%20%28single-precision%29))
  (Development|PrintString (Utilities|String|ToString(Float) (Variables|Default|GetCurrentLevel)) true true "(R=0.000000,G=0.660000,B=1.000000,A=1.000000)" DeltaSeconds))

(fn ConstructionScript)

(fn EnableSpawn
  (params (EnabledSpawn :type BP%20Spawner%20Object%20Reference) (bIsBeingEnabled :type Boolean)))

(fn StartSpawning
  (params (StartingSpawn :type BP%20Spawner%20Object%20Reference) (ExtraSpeed :type Float%20%28single-precision%29) (NumberOfEnemies :type Float%20%28single-precision%29) (TimeBetweenEnemies :type Float%20%28single-precision%29) (TimeBetweenWaves :type Float%20%28single-precision%29) (NumberOfWaves :type Float%20%28single-precision%29)))

(fn StartLevel
  (bind _currentlevel (Variables|Default|GetCurrentLevel))
  (Variables|LevelVariables|SetNumberOfWaves (Math|Float|Truncate (Math|Curves|GetFloatValue (Variables|Curves|GetCF_NumberOfWaves) _currentlevel)))
  (Variables|LevelVariables|SetCurrentEnemiesAddedSpeed (Math|Curves|GetFloatValue (Variables|Curves|GetCF_EnemiesAddedSpeed) _currentlevel))
  (Variables|LevelVariables|SetNumberOfEnemiesToFinish (Math|Float|Truncate (Math|Curves|GetFloatValue (Variables|Curves|GetCF_NumberOfEnemies) _currentlevel)))
  (Variables|LevelVariables|SetTimeBetweenEnemies (Math|Curves|GetFloatValue (Variables|Curves|GetCF_TimeBetweenEnemies) _currentlevel))
  (Variables|LevelVariables|SetTimeBetweenWaves (Math|Curves|GetFloatValue (Variables|Curves|GetCF_TimeBetweenWaves) _currentlevel))
  (for (_array_element _array_index) (Variables|Default|GetSpawns)
    (Utilities|Array|Insert (Variables|Default|GetbAreLevelsActiveArray) true _array_index)
    (Default|StartLevel _array_element (Variables|LevelVariables|GetCurrentEnemiesAddedSpeed) (Variables|LevelVariables|GetNumberOfEnemiesToFinish) (Variables|LevelVariables|GetNumberOfWaves) (Variables|LevelVariables|GetTimeBetweenEnemies) (Variables|LevelVariables|GetTimeBetweenWaves))
    (bind _asbp_input_manager_pawn (Utilities|Casting|CastToBP_InputManagerPawn (Pawn|GetControlledPawn (Game|GetPlayerController 0))))
    (Default|ShowStartLevelWidget (Variables|/Game/AEVIContent/BP_InputManagerPawn.BP_InputManagerPawn_C|GetHUDManager _asbp_input_manager_pawn))))

(fn LevelFinished
  (bind _asbp_aevijam_controller (Utilities|Casting|CastToBP_AEVIJamController (Game|GetPlayerController 0)))
  (Default|SetGameState _asbp_aevijam_controller "NewEnumerator1")
  (bind _asbp_input_manager_pawn (Utilities|Casting|CastToBP_InputManagerPawn (Pawn|GetControlledPawn (Game|GetPlayerController 0))))
  (Default|OnOleadaTerminada _asbp_input_manager_pawn)
  (Default|ShowEndLevelWidget (Variables|/Game/AEVIContent/BP_InputManagerPawn.BP_InputManagerPawn_C|GetHUDManager _asbp_input_manager_pawn)))

(fn SpawnLevelFinished
  (params (SpawnFinished :type BP%20Spawner%20Object%20Reference))
  (bind _barelevelsactivearray (Variables|Default|GetbAreLevelsActiveArray))
  (|SetBy-RefVar (Utilities|Array|Get(acopy) _barelevelsactivearray (Utilities|Array|FindItem (Variables|Default|GetSpawns) SpawnFinished)) false)
  (bind _array_element (Utilities|Array|ForEachLoopwithBreak _barelevelsactivearray :!label _label)
    (:LoopBody
      (if _array_element
        (goto _label Break)))
    (:Completed
      (CallFunction|LevelFinished)
      (Math|Float|IncrementFloat (Variables|Default|GetCurrentLevel)))))