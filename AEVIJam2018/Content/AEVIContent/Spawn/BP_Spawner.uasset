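; BP_Spawner is an enemy spawner actor whose StartLevel stores level settings and starts the first wave.
; StartWave sizes the wave as a geometric-growth share of the enemy total, then starts a looping SpawnEnemy timer.
; SpawnEnemy handles the Basic type by spawning BP_EnemyBase and adding the level's speed bonus to its walk speed.
; Nothing here stops the timer, enforces the wave count or advances to later waves.
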(event EventBeginPlay)

(event Collision|EventActorBeginOverlap
  (params (OtherActor :type Actor%20Object%20Reference)))

(event EventTick
  (params (DeltaSeconds :type Float%20%28single-precision%29)))

(fn ConstructionScript)

(fn StartLevel
  (params (EnemiesAddedSpeed :type Float%20%28single-precision%29) (NumberOfEnemies :type Float%20%28single-precision%29) (NumberOfWaves :type Float%20%28single-precision%29) (TimeBetweenEnemies :type Float%20%28single-precision%29) (TimeBetweenWaves :type Float%20%28single-precision%29))
  (LocalVariables|SetCurrentWave 1.0)
  (Variables|LevelVariables|SetEnemiesSpeedAdded EnemiesAddedSpeed)
  (Variables|LevelVariables|SetNumberOfWaves NumberOfWaves)
  (Variables|LevelVariables|SetNumberOfEnemies NumberOfEnemies)
  (Variables|LevelVariables|SetTimeBetweenEnemies TimeBetweenEnemies)
  (Variables|LevelVariables|SetTimeBetweenWaves TimeBetweenWaves)
  (CallFunction|StartWave (LocalVariables|GetCurrentWave)))

(fn StartWave
  (params (CurrentWave :type Float%20%28single-precision%29))
  (bind _output_get (LocalVariables|SetAuxWaveVar 0.0))
  (while (> CurrentWave _output_get)
    (LocalVariables|SetGrowthAccumulated (+ (LocalVariables|GetGrowthAccumulated) (Math|Float|Power (Variables|Default|GetGrowthPerWave) (LocalVariables|GetAuxWaveVar))))
    (Math|Float|IncrementFloat (LocalVariables|GetAuxWaveVar)))
  (LocalVariables|SetNumberOfEnemiesInWave (Math|Float|Ceil (* (/ (Math|Float|Power (Variables|Default|GetGrowthPerWave) (LocalVariables|GetAuxWaveVar)) (LocalVariables|GetGrowthAccumulated)) (Variables|LevelVariables|GetNumberOfEnemies))))
  (bind _returnvalue (Utilities|Time|SetTimerbyFunctionName 0 "SpawnEnemy" (Variables|LevelVariables|GetTimeBetweenEnemies) true))
  (Variables|Default|SetSpawnEnemyHandle _returnvalue))

(fn SpawnEnemy
  (switch Utilities|FlowControl|Switch|SwitchonEEnemyType (Variables|Default|GetEnemyType)
    (:NewEnumerator1
      (bind _returnvalue (Game|SpawnActorfromClass "/Game/AEVIContent/Enemies/BP_EnemyBase.BP_EnemyBase_C" (Math|Transform|MakeTransform "0, 0, 0" "0, 0, 0" "1,1,1") "AlwaysSpawn" 0 0))
      (Utilities|IsValid _returnvalue
        (:Is%20Valid
          (Variables|/Script/Engine.CharacterMovementComponent|SetMaxWalkSpeed (Variables|/Script/Engine.Character|GetCharacterMovement _returnvalue) (+ (Variables|/Script/Engine.CharacterMovementComponent|GetMaxWalkSpeed (Variables|/Script/Engine.Character|GetCharacterMovement _returnvalue)) (Variables|LevelVariables|GetEnemiesSpeedAdded))))
        (:Is%20Not%20Valid
          (Development|PrintString "Hello"))))))