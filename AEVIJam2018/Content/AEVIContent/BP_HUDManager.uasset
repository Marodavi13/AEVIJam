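; HUD manager Blueprint that puts phase timer, new wave, level start and level end widgets on the viewport.
; ShowTimer creates a counter widget with the given duration and binds its timer-ended callback to PhaseEnded, which prints a message and removes the widget.
; The wave and level events each create their widget, show it for a fixed three-second delay, then remove it.
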(event Custom|PhaseEnded
  (Development|PrintString "Phase Ended")
  (Widget|RemovefromParent (stale Custom|ShowTimer _returnvalue)))

(event Custom|ShowNewWaveWidget
  (bind _returnvalue (UserInterface|CreateWidget "/Game/AEVIContent/UI/BP_NewWave.BP_NewWave_C"))
  (UserInterface|Viewport|AddtoViewport _returnvalue 0)
  (Utilities|FlowControl|Delay 3.0)
  (Widget|RemovefromParent _returnvalue))

(event Custom|ShowStartLevelWidget
  (bind _returnvalue (UserInterface|CreateWidget "/Game/AEVIContent/UI/BP_StartLevelWidget.BP_StartLevelWidget_C"))
  (UserInterface|Viewport|AddtoViewport _returnvalue 0)
  (Utilities|FlowControl|Delay 3.0)
  (Widget|RemovefromParent _returnvalue))

(event Custom|ShowTimer
  (params (Duration :type Float%20%28single-precision%29))
  (bind _returnvalue (UserInterface|CreateWidget "/Game/AEVIContent/UI/BP_CounterWidget.BP_CounterWidget_C"))
  (Variables|/Game/AEVIContent/UI/BP_CounterWidget.BP_CounterWidget_C|SetMaxTime _returnvalue Duration)
  (UserInterface|Viewport|AddtoViewport _returnvalue 0)
  (EventDispatchers|BindEventtoWidgetTimerEnded _returnvalue (delegate Custom|PhaseEnded)))

(event Custom|ShowEndLevelWidget
  (bind _returnvalue (UserInterface|CreateWidget "/Game/AEVIContent/UI/BP_EndLevelWidget.BP_EndLevelWidget_C"))
  (UserInterface|Viewport|AddtoViewport _returnvalue 0)
  (Utilities|FlowControl|Delay 3.0)
  (Widget|RemovefromParent _returnvalue))

(event EventBeginPlay)

(fn ConstructionScript)