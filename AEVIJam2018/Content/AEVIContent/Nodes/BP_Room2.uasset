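; BP_Room2 is an interactable room node that either opens an upgrade menu or applies a used skill to enemies inside its box.
; Interact with no skill creates BP_Upgrade with itself as calling node; the three upgrade events only print placeholders.
; Otherwise it constructs the skill class and casts to identify it: Nuke destroys all overlapping enemies, Binary Ray randomly destroys one of two enemy types.
; Decoy briefly enables a visible, collidable sphere and prints overlapping enemy names.
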(event Custom|Upgrade3
  (Development|PrintString "Upgrade3"))

(event Custom|Upgrade2
  (Development|PrintString "Upgrade2"))

(event Custom|Upgrade1
  (Development|PrintString "Upgrade1"))

(event EventBeginPlay)

(event Collision|EventActorBeginOverlap
  (params (OtherActor :type Actor%20Object%20Reference)))

(event EventTick
  (params (DeltaSeconds :type Float%20%28single-precision%29)))

(event EventInteract
  (params (SkillUsed :type BP%20Skill%20Class%20Reference))
  (bind _sphere (Variables|Default|GetSphere))
  (bind _sphere_2 (Variables|Default|GetSphere))
  (if (== SkillUsed 0)
    ;[1 1 1] Mejora
    (Development|PrintString "Interactuando")
    (bind _returnvalue (UserInterface|CreateWidget "/Game/AEVIContent/UI/BP_Upgrade.BP_Upgrade_C" (Game|GetPlayerController 0)))
    (Variables|/Game/AEVIContent/UI/BP_Upgrade.BP_Upgrade_C|SetCallingNode _returnvalue self)
    (UserInterface|Viewport|AddtoViewport _returnvalue 0)
    (else
      (bind _returnvalue_2 (Game|ConstructObjectfromClass SkillUsed self))
      (Utilities|Casting|CastToBP_SkillNuke _returnvalue_2
        (:then
          ;[1 1 1] Nuke
          (bind _arrayelement (Utilities|Array|ReverseforEachLoop (Collision|GetOverlappingActors (Variables|Default|GetBox%20Collision) "/Game/AEVIContent/Enemies/BP_EnemyBase.BP_EnemyBase_C" :!class /Script/Engine.PrimitiveComponent))
            (:LoopBody
              (Actor|DestroyActor _arrayelement))))
        (:CastFailed
          ;[1 1 1] Binary Ray
          (Utilities|Casting|CastToBP_SkillBinaryRay _returnvalue_2
            (:then
              (if (<= (Math|Random|RandomIntegerinRange 1 100) 50)
                (bind _arrayelement_2 (Utilities|Array|ReverseforEachLoop (Collision|GetOverlappingActors (Variables|Default|GetBox%20Collision) "/Game/AEVIContent/Enemies/BP_Enemy0.BP_Enemy0_C" :!class /Script/Engine.PrimitiveComponent))
                  (:LoopBody
                    (Actor|DestroyActor _arrayelement_2)))
                (else
                  (bind _arrayelement_3 (Utilities|Array|ReverseforEachLoop (Collision|GetOverlappingActors (Variables|Default|GetBox%20Collision) "/Game/AEVIContent/Enemies/BP_Enemy1.BP_Enemy1_C" :!class /Script/Engine.PrimitiveComponent))
                    (:LoopBody
                      (Actor|DestroyActor _arrayelement_3))))))
            (:CastFailed
              ;[1 1 1] Decoy
              (Utilities|Casting|CastToBP_SkillDecoy _returnvalue_2)
              (Development|SetHiddeninGame _sphere_2 false false)
              (Collision|SetCollisionEnabled _sphere_2 "QueryAndPhysics")
              (bind _arrayelement_4 (Utilities|Array|ReverseforEachLoop (Collision|GetOverlappingActors (Variables|Default|GetBox%20Collision) "/Game/AEVIContent/Enemies/BP_EnemyBase.BP_EnemyBase_C" :!class /Script/Engine.PrimitiveComponent))
                (:LoopBody
                  (Development|PrintString (Utilities|GetDisplayName _arrayelement_4)))
                (:Completed
                  (Utilities|FlowControl|Delay 4.0)
                  (Development|SetHiddeninGame _sphere true false)
                  (Collision|SetCollisionEnabled _sphere "NoCollision"))))))))))

(fn ConstructionScript
  (|CallParentFunction))