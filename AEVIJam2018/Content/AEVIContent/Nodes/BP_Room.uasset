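; Room actor that applies a player skill to the enemies overlapping its collision box through an Interact event.
; It instantiates the passed skill class and branches through a cast chain.
; Nuke destroys all enemies, while Binary Ray randomly destroys one of two enemy types.
; Decoy temporarily enables a visible, collidable sphere, and Push launches enemies toward an earlier entry in their LastPositions using a computed velocity.
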(event EventBeginPlay)

(event Collision|EventActorBeginOverlap
  (params (OtherActor :type Actor%20Object%20Reference)))

(event EventTick
  (params (DeltaSeconds :type Float%20%28single-precision%29)))

(event EventInteract
  (params (SkillUsed :type BP%20Skill%20Class%20Reference))
  (bind _launchtime (Variables|Push|GetLaunchTime))
  (bind _sphere (Variables|Default|GetSphere))
  (bind _sphere_2 (Variables|Default|GetSphere))
  (bind _returnvalue (Game|ConstructObjectfromClass SkillUsed self))
  (Utilities|Casting|CastToBP_SkillNuke _returnvalue
    (:then
      ;[1 1 1] Nuke
      (bind _arrayelement (Utilities|Array|ReverseforEachLoop (Collision|GetOverlappingActors (Variables|Default|GetBox%20Collision) "/Game/AEVIContent/Enemies/BP_EnemyBase.BP_EnemyBase_C" :!class /Script/Engine.PrimitiveComponent))
        (:LoopBody
          (Actor|DestroyActor _arrayelement))))
    (:CastFailed
      ;[1 1 1] Binary Ray
      (Utilities|Casting|CastToBP_SkillBinaryRay _returnvalue
        (:then
          (if (<= (Math|Random|RandomIntegerinRange 1 100) 50)
            (bind _arrayelement_2 (Utilities|Array|ReverseforEachLoop (Collision|GetOverlappingActors (Variables|Default|GetBox%20Collision) "/Game/AEVIContent/Enemies/BP_Enemy0.BP_Enemy0_C" :!class /Script/Engine.PrimitiveComponent))
              (:LoopBody
                (Actor|DestroyActor _arrayelement_2)))
            (else
              (bind _arrayelement_3 (Utilities|Array|ReverseforEachLoop (Collision|GetOverlappingActors (Variables|Default|GetBox%20Collision) "/Game/AEVIContent/Enemies/BP_Enemy1.BP_Enemy1_C" :!class /Script/Engine.PrimitiveComponent))
                (:LoopBody
                  (Actor|DestroyActor _arrayelement_3))))))
        (:CastFailed
          ;[1 1 1] Decoy
          (Utilities|Casting|CastToBP_SkillDecoy _returnvalue
            (:then
              (Development|SetHiddeninGame _sphere_2 false false)
              (Collision|SetCollisionEnabled _sphere_2 "QueryAndPhysics")
              (bind _arrayelement_4 (Utilities|Array|ReverseforEachLoop (Collision|GetOverlappingActors (Variables|Default|GetBox%20Collision) "/Game/AEVIContent/Enemies/BP_EnemyBase.BP_EnemyBase_C" :!class /Script/Engine.PrimitiveComponent))
                (:LoopBody
                  (Development|PrintString (Utilities|GetDisplayName _arrayelement_4)))
                (:Completed
                  (Utilities|FlowControl|Delay 4.0)
                  (Development|SetHiddeninGame _sphere true false)
                  (Collision|SetCollisionEnabled _sphere "NoCollision"))))
            (:CastFailed
              ;[1 1 1] Push
              (Utilities|Casting|CastToBP_SkillPush _returnvalue)
              (bind _arrayelement_5 (Utilities|Array|ReverseforEachLoop (Collision|GetOverlappingActors (Variables|Default|GetBox%20Collision) "/Game/AEVIContent/Enemies/BP_EnemyBase.BP_EnemyBase_C" :!class /Script/Engine.PrimitiveComponent))
                (:LoopBody
                  (bind _asbp_enemy_base (Utilities|Casting|CastToBP_EnemyBase _arrayelement_5))
                  (Character|LaunchCharacter _asbp_enemy_base (- (/ (- (Transformation|GetActorLocation (Utilities|Array|Get(acopy) (Variables|/Game/AEVIContent/Enemies/BP_EnemyBase.BP_EnemyBase_C|GetLastPositions _asbp_enemy_base) (- (Variables|Push|GetPushBackPositions) 1))) (Transformation|GetActorLocation _arrayelement_5)) _launchtime) (* (* (Class|Actor|GetInputVectorAxisValue) _launchtime) 0.5)) false false))))))))))

(fn ConstructionScript
  (|CallParentFunction))