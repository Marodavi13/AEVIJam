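; BP_Connection is a connection node that accepts player upgrades and skills.
; Its construction script picks the mesh from Type and toggles the down and right meshes' visibility and collision for non-4-way shapes.
; Interact either opens the upgrade widget or constructs and activates the given Nuke, Binary Ray, Decoy or Push skill on itself.
; Upgrade events apply SlowDown or Trap objects; Upgrade3 only prints, leaving Wall unwired.
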(event Custom|SetMeshVisibility
  (params (Mesh :type Static%20Mesh%20Component%20Object%20Reference) (bVisibility :type Boolean))
  ;[1 1 1] SetUnusedVisibily
  (Rendering|SetVisibility Mesh bVisibility false)
  (if bVisibility
    (Collision|SetCollisionEnabled Mesh "QueryAndPhysics")
    (else
      (Collision|SetCollisionEnabled Mesh "NoCollision"))))

(event Custom|Interact
  (params (SkillUsed :type BP%20Skill%20Class%20Reference))
  (if (== SkillUsed 0)
    ;[1 1 1] Mejora
    (Development|PrintString "Interactuando")
    (bind _returnvalue (UserInterface|CreateWidget "/Game/AEVIContent/UI/BP_UpgradeWidget.BP_UpgradeWidget_C" (Game|GetPlayerController 0)))
    (Variables|/Game/AEVIContent/UI/BP_UpgradeWidget.BP_UpgradeWidget_C|SetCallingNode _returnvalue self)
    (UserInterface|Viewport|AddtoViewport _returnvalue 0)
    (else
      (bind _returnvalue_2 (Game|ConstructObjectfromClass SkillUsed self))
      (bind _asbp_skill_nuke (Utilities|Casting|CastToBP_SkillNuke _returnvalue_2)
        (:then
          ;[1 1 1] Nuke
          (Variables|/Game/AEVIContent/Skillz/BP_Skill.BP_Skill_C|SetNode _asbp_skill_nuke self)
          (Default|ActivateSkill _asbp_skill_nuke))
        (:CastFailed
          ;[1 1 1] Binary Ray
          (bind _asbp_skill_binary_ray (Utilities|Casting|CastToBP_SkillBinaryRay _returnvalue_2)
            (:then
              (Variables|/Game/AEVIContent/Skillz/BP_Skill.BP_Skill_C|SetNode _asbp_skill_binary_ray self)
              (Default|ActivateSkill _asbp_skill_binary_ray))
            (:CastFailed
              ;[1 1 1] Decoy
              (bind _asbp_skill_decoy (Utilities|Casting|CastToBP_SkillDecoy _returnvalue_2)
                (:then
                  (Variables|/Game/AEVIContent/Skillz/BP_Skill.BP_Skill_C|SetNode _asbp_skill_decoy self)
                  (Default|ActivateSkill _asbp_skill_decoy))
                (:CastFailed
                  ;[1 1 1] Push
                  (bind _asbp_skill_push (Utilities|Casting|CastToBP_SkillPush _returnvalue_2))
                  (Variables|/Game/AEVIContent/Skillz/BP_Skill.BP_Skill_C|SetNode _asbp_skill_push self)
                  (Default|ActivateSkill _asbp_skill_push))))))))))

(event EventUpgrade1
  ;[1 1 1] Upgrades
  (Development|PrintString "UpgradeRoom1")
  (bind _returnvalue (Game|ConstructObjectfromClass "/Game/AEVIContent/Upgrades/ConnectionUpgrades/BP_Upgrade_Connection_SlowDown.BP_Upgrade_Connection_SlowDown_C" (Game|GetPlayerController 0)))
  (Variables|/Game/AEVIContent/Upgrades/BP_Upgrade.BP_Upgrade_C|SetNode _returnvalue self)
  (Default|ActivateUpgrade _returnvalue))

(event Collision|EventActorBeginOverlap
  (params (OtherActor :type Actor%20Object%20Reference)))

(event EventTick
  (params (DeltaSeconds :type Float%20%28single-precision%29)))

(event EventUpgrade2
  ;[1 1 1] Upgrades
  (Development|PrintString "UpgradeRoom2")
  (bind _returnvalue (Game|ConstructObjectfromClass "/Game/AEVIContent/Upgrades/ConnectionUpgrades/BP_Upgrade_Connection_Trap.BP_Upgrade_Connection_Trap_C" (Game|GetPlayerController 0)))
  (Variables|/Game/AEVIContent/Upgrades/BP_Upgrade.BP_Upgrade_C|SetNode _returnvalue self)
  (Default|ActivateUpgrade _returnvalue))

(event EventUpgrade3
  ;[1 1 1] Upgrades
  (Development|PrintString "UpgradeRoom3"))

(fn ConstructionScript
  (bind _staticmesh (Variables|Default|GetStaticMesh))
  (|CallParentFunction)
  (switch Utilities|FlowControl|Switch|SwitchonEConnectionType (Variables|Default|GetType)
    (:NewEnumerator0
      (Components|StaticMesh|SetStaticMesh _staticmesh "/Game/AEVIContent/Art/Meshes/SM_Connection_Straight.SM_Connection_Straight")
      (CallFunction|SetMeshVisibility (Variables|Default|GetStaticMeshDown) false)
      (CallFunction|SetMeshVisibility (Variables|Default|GetStaticMeshRight) true))
    (:NewEnumerator1
      (Components|StaticMesh|SetStaticMesh _staticmesh "/Game/AEVIContent/Art/Meshes/SM_Connection_T.SM_Connection_T")
      (CallFunction|SetMeshVisibility (Variables|Default|GetStaticMeshDown) true)
      (CallFunction|SetMeshVisibility (Variables|Default|GetStaticMeshRight) true))
    (:NewEnumerator3
      (Components|StaticMesh|SetStaticMesh _staticmesh "/Game/AEVIContent/Art/Meshes/SM_Connection_L.SM_Connection_L")
      (CallFunction|SetMeshVisibility (Variables|Default|GetStaticMeshDown) true)
      (CallFunction|SetMeshVisibility (Variables|Default|GetStaticMeshRight) false))
    (:NewEnumerator4
      (Components|StaticMesh|SetStaticMesh _staticmesh "/Game/Geometry/Meshes/1M_Cube.1M_Cube"))))